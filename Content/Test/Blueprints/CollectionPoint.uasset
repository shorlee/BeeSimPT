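; CollectionPoint is a Blueprint for a resource node that can be drained and refilled, kept in a test folder.
; Drain zeroes ResourceAmount, sets IsDrained and prints the stored resource's name as debug text.
; Refill clears the flag and restores the amount to one, and each function acts only when the flag is in the opposite state.
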(fn Drain
  (if (not (Variables|Default|GetisDrained))
    (Variables|Default|SetresourceAmount 0.0)
    (Variables|Default|SetisDrained true)
    ;[1 1 1] DEBUG
    (Development|PrintString (Utilities|String|Append "Drained: " (Utilities|String|ToString(Name) (Variables|/Game/Test/Blueprints/Resource.Resource_C|Getname (Variables|Default|Getresource_Stored)))) true false "(R=0.863357,G=1.000000,B=0.000000,A=1.000000)")))

(fn Refill
  (if (Variables|Default|GetisDrained)
    (Variables|Default|SetisDrained false)
    (Variables|Default|SetresourceAmount 1.0)))