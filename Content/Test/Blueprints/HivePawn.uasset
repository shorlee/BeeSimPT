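; Hive pawn that takes over player control when another pawn overlaps its trigger, showing the mouse cursor.
; Interact hands possession back to the stored previous pawn, while a lock blocks re-possession until that pawn leaves the trigger.
; Yaw and Pitch axes rotate the spring arm by mouse sensitivity, with pitch limited to a maximum angle.
; Left mouse sets a Turning flag that nothing here reads yet.
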(event OnComponentBeginOverlap(Trigger)
  (params (OverlappedComponent :type Primitive%20Component%20Object%20Reference) (OtherActor :type Actor%20Object%20Reference) (OtherComp :type Primitive%20Component%20Object%20Reference) (OtherBodyIndex :type Integer) (bFromSweep :type Boolean) (SweepResult :type Hit%20Result%20Structure%20%28by%20ref%29))
  (bind _returnvalue (Game|GetPlayerController 0))
  ;[1 1 1] StartPosession
  (bind _aspawn (Utilities|Casting|CastToPawn OtherActor))
  (if (not (Variables|Default|GetisLocked))
    (Variables|Default|SetpreviousPawn _aspawn)
    (if (not (Pawn|IsPlayerControlled))
      (Pawn|Possess _returnvalue self)
      (Variables|/Script/Engine.PlayerController|SetbShowMouseCursor _returnvalue true)
      (Variables|Default|SetisLocked true))))

(event OnComponentEndOverlap(Trigger)
  (params (OverlappedComponent :type Primitive%20Component%20Object%20Reference) (OtherActor :type Actor%20Object%20Reference) (OtherComp :type Primitive%20Component%20Object%20Reference) (OtherBodyIndex :type Integer))
  ;[1 1 1] unlock
  (if (== OtherActor (Variables|Default|GetpreviousPawn))
    (Variables|Default|SetisLocked false)))

(event Input|ActionEvents|InputActionInteract
  (params (Key :type Key%20Structure))
  (bind _returnvalue (Game|GetPlayerController 0))
  (bind _previouspawn (Variables|Default|GetpreviousPawn))
  ;[1 1 1] Stop Possession to possess previous
  (:Pressed
    (if (Pawn|IsPlayerControlled)
      (Utilities|IsValid _previouspawn
        (:Is%20Valid
          (Pawn|Possess _returnvalue _previouspawn)
          (Variables|/Script/Engine.PlayerController|SetbShowMouseCursor _returnvalue false))
        (:Is%20Not%20Valid
          (Development|PrintString "INVALID PAWN"))))))

(event Input|AxisEvents|InputAxisPitch
  (params (AxisValue :type Float%20%28single-precision%29))
  (bind _maxvertrotation (Variables|Default|GetmaxVertRotation))
  (bind _maxvertrotation_2 (Variables|Default|GetmaxVertRotation))
  (bind _springarm (Variables|Default|GetSpringArm))
  (bind _returnvalue (Transformation|GetWorldRotation _springarm))
  (bind _returnvalue_2 (* _maxvertrotation -1.0))
  (bind (_roll _pitch _yaw) (Math|Rotator|BreakRotator _returnvalue))
  (bind _returnvalue_3 (< _pitch _maxvertrotation))
  (bind _returnvalue_4 (> _pitch _returnvalue_2))
  (bind _returnvalue_5 (and _returnvalue_3 _returnvalue_4))
  ;[1 1 1] Controls
  (if _returnvalue_5
    (Transformation|AddRelativeRotation (Variables|Default|GetSpringArm) (Math|Vector|RotatorfromAxisandAngle "0,1.000000,0.000000" (* AxisValue (Variables|Default|GetMouseSens))) true false)
    ;;[1 0.381 0.1947] Limit Rotation
    (if (not _returnvalue_5)
      (if (> _pitch 0.0)
        (Transformation|SetRelativeRotation _springarm (Math|Rotator|MakeRotator 0.0 _maxvertrotation_2 _yaw) false false)
        (else
          (Transformation|SetRelativeRotation _springarm (Math|Rotator|MakeRotator 0.0 (* _maxvertrotation_2 -1.0) _yaw) false false))))))

(event Input|AxisEvents|InputAxisYaw
  (params (AxisValue :type Float%20%28single-precision%29))
  ;[1 1 1] Controls
  (Transformation|AddRelativeRotation (Variables|Default|GetSpringArm) (Math|Vector|RotatorfromAxisandAngle "0, 0,1.000000" (* AxisValue (Variables|Default|GetMouseSens))) true false))

(event Input|MouseEvents|LeftMouseButton
  (params (Key :type Key%20Structure))
  ;[1 1 1] Controls
  ;;[1 1 1] For later possibly
  (:Pressed
    (Variables|Default|Setturning true))
  (:Released
    (Variables|Default|Setturning false)))

(fn ConstructionScript)