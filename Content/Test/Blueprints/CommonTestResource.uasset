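; CommonTestResource is a test resource actor that the player's FlyingPawn can drain by interacting nearby.
; The construction script picks the mesh from the resource list by ResourceID and MeshVariant, and assigns that ID to every CollectionPoint component.
; On BeginPlay it binds to the controlled pawn's interact event.
; A gate, opened and closed by Trigger1 overlaps without filtering the overlapping actor, controls whether interaction drains CollectionPoint1.
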(event OnComponentBeginOverlap(Trigger1)
  (params (OverlappedComponent :type Primitive%20Component%20Object%20Reference) (OtherActor :type Actor%20Object%20Reference) (OtherComp :type Primitive%20Component%20Object%20Reference) (OtherBodyIndex :type Integer) (bFromSweep :type Boolean) (SweepResult :type Hit%20Result%20Structure%20%28by%20ref%29))
  ;[1 1 1] Interaction with CollectionPoint1
  (Utilities|FlowControl|Gate true) ; enters at Open
)

(event OnComponentEndOverlap(Trigger1)
  (params (OverlappedComponent :type Primitive%20Component%20Object%20Reference) (OtherActor :type Actor%20Object%20Reference) (OtherComp :type Primitive%20Component%20Object%20Reference) (OtherBodyIndex :type Integer))
  ;[1 1 1] Interaction with CollectionPoint1
  (Utilities|FlowControl|Gate true) ; enters at Close
)

(event Custom|InteractionByFlyingBP
  ;[1 1 1] Interaction with CollectionPoint1
  (Utilities|FlowControl|Gate true
    (:Exit
      (Default|Drain (Variables|Default|GetCollectionPoint1)))))

(event EventBeginPlay
  ;[1 1 1] bind event
  (bind _asflying_pawn (Utilities|Casting|CastToFlyingPawn (Pawn|GetControlledPawn (Game|GetPlayerController 0))))
  (EventDispatchers|BindEventtoInteract _asflying_pawn (delegate Custom|InteractionByFlyingBP)))

(fn ConstructionScript
  (bind _meshvariant (CallFunction|GetResourceList))
  (Components|StaticMesh|SetStaticMesh (Variables|Default|GetPH_mesh) (Utilities|Array|Get(acopy) (Utilities|Struct|BreakMeshChooser (Utilities|Array|Get(acopy) _meshvariant (Variables|Default|GetResourceID))) (Variables|Default|GetMeshVariant)))
  (for _array_element (Actor|GetComponentsByClass "/Game/Test/Blueprints/CollectionPoint.CollectionPoint_C")
    (Variables|/Game/Test/Blueprints/CollectionPoint.CollectionPoint_C|Setresource_Stored _array_element (Variables|Default|GetResourceID))))